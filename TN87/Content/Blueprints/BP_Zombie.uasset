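; BP_Zombie is an enemy that chases the player, attacks up close and may drop ammo or a medkit on death.
; BeginPlay randomly picks a Giga variant via the anim Blueprint, making the others slower and weaker, and starts a self-recursing random groan loop.
; Tick reissues AIMoveTo while alive; arrival triggers a DoOnce-gated, delayed sphere-trace hit.
; Depleted health stops it, plays death, rolls drops and later destroys it.
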(event Custom|HandleDeath
  ;[1 1 1] Handle Death
  (Variables|Default|SetAlive false)
  (Components|Movement|StopMovementImmediately (Variables|Character|GetCharacterMovement))
  (Components|Animation|PlayAnimation (Variables|Character|GetMesh) "/Game/Mesh/Zombie/Animation/Zombie_Death.Zombie_Death" false)
  (Collision|SetCollisionEnabled (Variables|Collision|GetCapsuleComponent) "NoCollision")
  (CallFunction|HandleDrops)
  (Utilities|FlowControl|Delay 2e+01)
  (Actor|DestroyActor))

(event Custom|HandleDrops
  (bind _returnvalue (Transformation|GetActorTransform))
  ;[1 1 1] Handle Drops
  (if (== (Math|Random|RandomIntegerinRange 0 2) 0)
    (if (Math|Random|RandomBool)
      (Game|SpawnActorfromClass "/Game/Blueprints/BP_AmmoPickup.BP_AmmoPickup_C" _returnvalue "Undefined" 0 0)
      (else
        (Game|SpawnActorfromClass "/Game/Blueprints/BP_Medkit.BP_Medkit_C" _returnvalue "Undefined" 0 0)))))

(event Custom|Raycast
  (bind _capsulecomponent (Variables|Collision|GetCapsuleComponent))
  (bind _returnvalue (Transformation|GetWorldLocation _capsulecomponent))
  ;[1 1 1] Raycast
  (bind (_outhit _returnvalue_2) (Collision|SphereTraceForObjects _returnvalue (+ _returnvalue (* (Math|Vector|GetForwardVector (Transformation|GetWorldRotation _capsulecomponent)) 75.0)) 75.0 (Utilities|Array|MakeArray "ObjectTypeQuery3") false 0 "None"))
  (if _returnvalue_2
    (if (== (.HitActor (Collision|BreakHitResult _outhit)) (Variables|Default|GetPlayer))
      (Game|Damage|ApplyDamage (.HitActor (Collision|BreakHitResult _outhit)) (Variables|Default|GetBase%20Damage) 0 0))))

(event Custom|MakeZombieNoise
  ;[1 1 1] Zombie Audio
  (Utilities|FlowControl|Delay (Math|Random|RandomFloatinRange 1.0 12.0))
  (if (Variables|Default|GetAlive)
    (Audio|PlaySoundatLocation "/Game/Audio/Zombie/ZombieCue.ZombieCue" (Transformation|GetActorLocation) "0, 0, 0" (Math|Random|RandomFloatinRange 0.25 1.0) (Math|Random|RandomFloatinRange 0.1 1.0) 0.0 0 0 0)
    (if (Variables|Default|GetAlive)
      (CallFunction|MakeZombieNoise))))

(event EventBeginPlay
  (bind _charactermovement (Variables|Character|GetCharacterMovement))
  ;[1 1 1] Giga Zombie%
  (Utilities|FlowControl|Sequence
    (:then_0
      (bind _asabp_zombie (Utilities|Casting|CastToABP_Zombie (Components|SkeletalMesh|GetAnimInstance (Variables|Character|GetMesh))))
      (bind _output_get (Variables|/Game/Mesh/Zombie/Animation/ABP_Zombie.ABP_Zombie_C|SetGiga%20Zombie _asabp_zombie (Math|Random|RandomBool)))
      (bind _output_get_2 (Variables|Default|SetGigaZombie _output_get))
      (if (not _output_get_2)
        (Variables|/Script/Engine.CharacterMovementComponent|SetMaxWalkSpeed _charactermovement (/ (Variables|/Script/Engine.CharacterMovementComponent|GetMaxWalkSpeed _charactermovement) 5.0))
        (Variables|Default|SetHealth (- (Variables|Default|GetHealth) 1e+01))))
    (:then_1
      ;[1 1 1] Get Player Ref
      (bind _asfirst_person_character (Utilities|Casting|CastToFirstPersonCharacter (Game|GetPlayerCharacter 0)))
      (Variables|Default|SetPlayer _asfirst_person_character)
      ;[1 1 1] Init Zombie Noise
      (CallFunction|MakeZombieNoise))))

(event Game|Damage|EventAnyDamage
  (params (Damage :type Float%20%28single-precision%29) (DamageType :type Damage%20Type%20Object%20Reference) (InstigatedBy :type Controller%20Object%20Reference) (DamageCauser :type Actor%20Object%20Reference))
  ;[1 1 1] Handle Damage
  (bind _output_get (Variables|Default|SetHealth (- (Variables|Default|GetHealth) Damage)))
  (if (<= _output_get 0.0)
    (Utilities|FlowControl|DoOnce false
      (:Completed
        (CallFunction|HandleDeath)))))

(event EventTick
  (params (DeltaSeconds :type Float%20%28single-precision%29))
  ;[1 1 1] FSM
  (if (Variables|Default|GetAlive)
    (AI|AIMoveTo self "0, 0, 0" (Variables|Default|GetPlayer) 5.0 true
      (:OnSuccess
        (Utilities|FlowControl|DoOnce false :!label _label
          (:Completed
            (Variables|Default|SetIsAttacking true)
            (Utilities|FlowControl|RetriggerableDelay 0.75)
            (CallFunction|Raycast)
            (Utilities|FlowControl|RetriggerableDelay 1.0)
            (Variables|Default|SetIsAttacking false)
            (goto _label Reset)))))))

(fn ConstructionScript)