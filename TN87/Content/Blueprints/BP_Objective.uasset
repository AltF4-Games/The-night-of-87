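; BP_Objective is a trigger volume that hands the player a new objective when they walk into it.
; On overlap with the FirstPersonCharacter, it passes its objective and time to the character, then destroys itself so it fires once.
; When TriggerStartWalk is set, it also finds the first BP_Ghost in the level and enables its walking before destruction.
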(event OnComponentBeginOverlap(Box)
  (params (OverlappedComponent :type Primitive%20Component%20Object%20Reference) (OtherActor :type Actor%20Object%20Reference) (OtherComp :type Primitive%20Component%20Object%20Reference) (OtherBodyIndex :type Integer) (bFromSweep :type Boolean) (SweepResult :type Hit%20Result%20Structure%20%28by%20ref%29))
  ;[1 1 1] Objective Trigger
  (bind _asfirst_person_character (Utilities|Casting|CastToFirstPersonCharacter OtherActor))
  (Default|SetObjective _asfirst_person_character (Variables|Default|GetObjective) (Variables|Default|GetTime))
  (if (Variables|Default|GetTriggerStartWalk)
    (CallFunction|StartWalk)
    (Actor|DestroyActor)
    (else
      (Actor|DestroyActor))))

(event Custom|StartWalk
  ;[1 1 1] Start Walk
  (bind _outactors (Actor|GetAllActorsOfClass "/Game/Blueprints/BP_Ghost.BP_Ghost_C"))
  (Utilities|IsValid (Utilities|Array|Get(acopy) _outactors)
    (:Is%20Valid
      (Variables|/Game/Blueprints/BP_Ghost.BP_Ghost_C|SetCanWalk (Utilities|Array|Get(acopy) _outactors) true))))

(fn ConstructionScript)