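; Trigger-volume spawner that creates a group of BP_Zombie AI when the player walks into it.
; BeginPlay gathers the spawn point components into an array.
; The first box overlap by a FirstPersonCharacter passes a DoOnce gate and spawns one zombie at each point's world location.
; The spawner then destroys itself, so it fires only once.
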(event OnComponentBeginOverlap(Box)
  (params (OverlappedComponent :type Primitive%20Component%20Object%20Reference) (OtherActor :type Actor%20Object%20Reference) (OtherComp :type Primitive%20Component%20Object%20Reference) (OtherBodyIndex :type Integer) (bFromSweep :type Boolean) (SweepResult :type Hit%20Result%20Structure%20%28by%20ref%29))
  (bind _spawnpoints (Variables|Default|GetSpawnPoints))
  ;[1 1 1] Spawn AI's
  (Utilities|Casting|CastToFirstPersonCharacter OtherActor)
  (Utilities|FlowControl|DoOnce false
    (:Completed
      (for (_ _array_index) _spawnpoints
        (AI|SpawnAIFromClass "/Game/Blueprints/BP_Zombie.BP_Zombie_C" 0 (Transformation|GetWorldLocation (Utilities|Array|Get(acopy) _spawnpoints _array_index)) "0, 0, 0" false 0))
      (Actor|DestroyActor))))

(event EventBeginPlay
  ;[1 1 1] Make Spawn Point Array
  (Variables|Default|SetSpawnPoints (Utilities|Array|MakeArray (Variables|Default|GetSpawn%20Point%208) (Variables|Default|GetSpawn%20Point%204) (Variables|Default|GetSpawn%20Point%201) (Variables|Default|GetSpawn%20Point%202) (Variables|Default|GetSpawn%20Point%203) (Variables|Default|GetSpawn%20Point%209) (Variables|Default|GetSpawn%20Point%205) (Variables|Default|GetSpawn%20Point%206) (Variables|Default|GetSpawn%20Point%207) (Variables|Default|GetSpawn%20Point%2011) (Variables|Default|GetSpawn%20Point%2012))))

(fn ConstructionScript)