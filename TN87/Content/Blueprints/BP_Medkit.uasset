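; Health pickup actor that restores health to the first-person player character on overlap.
; Each tick the static mesh spins in yaw at a configurable speed.
; When a FirstPersonCharacter enters the box, it plays a pickup sound, adds health clamped to the player's maximum, updates the player's HUD value, then destroys itself.
; A DoOnce gate keeps the pickup from triggering more than once.
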(event OnComponentBeginOverlap(Box)
  (params (OverlappedComponent :type Primitive%20Component%20Object%20Reference) (OtherActor :type Actor%20Object%20Reference) (OtherComp :type Primitive%20Component%20Object%20Reference) (OtherBodyIndex :type Integer) (bFromSweep :type Boolean) (SweepResult :type Hit%20Result%20Structure%20%28by%20ref%29))
  ;[1 1 1] Pickup Health
  (bind _asfirst_person_character (Utilities|Casting|CastToFirstPersonCharacter OtherActor))
  (Variables|Default|SetPlayer _asfirst_person_character)
  (Utilities|FlowControl|DoOnce false
    (:Completed
      (Audio|PlaySound2D "/Game/Audio/Item_Pickup.Item_Pickup" 1.0 1.0 0.0 0 0)
      (bind _output_get (Variables|/Game/FirstPersonBP/FirstPersonCharacter.FirstPersonCharacter_C|SetHealth (Variables|Default|GetPlayer) (Math|Float|Clamp(Float) (+ (Variables|/Game/FirstPersonBP/FirstPersonCharacter.FirstPersonCharacter_C|GetHealth (Variables|Default|GetPlayer)) (Variables|Default|GetHealthToAdd)) 0.0 (Variables|/Game/FirstPersonBP/FirstPersonCharacter.FirstPersonCharacter_C|GetMaxHealth (Variables|Default|GetPlayer)))))
      (Variables|/Game/UI/WBP_HUD.WBP_HUD_C|SetHealth (Variables|/Game/FirstPersonBP/FirstPersonCharacter.FirstPersonCharacter_C|GetHUD (Variables|Default|GetPlayer)) _output_get)
      (Actor|DestroyActor))))

(event EventTick
  (params (DeltaSeconds :type Float%20%28single-precision%29))
  ;[1 1 1] Rotate Mesh
  (Transformation|AddRelativeRotation (Variables|Default|GetStaticMesh) (Math|Rotator|MakeRotator 0.0 0.0 (* DeltaSeconds (Variables|Default|GetSpeed))) false false))

(fn ConstructionScript)