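; BP_AmmoPickup is a spinning ammo pickup that adds one clip to a Glock when the first-person character touches it.
; Tick rotates the mesh around yaw at a frame-rate-independent Speed.
; A box overlap passes a character cast and DoOnce, then plays the pickup sound and increments Clips on the first BP_Glock found via GetAllActorsOfClass.
; The pickup destroys itself whether or not a valid Glock exists.
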(event OnComponentBeginOverlap(Box)
  (params (OverlappedComponent :type Primitive%20Component%20Object%20Reference) (OtherActor :type Actor%20Object%20Reference) (OtherComp :type Primitive%20Component%20Object%20Reference) (OtherBodyIndex :type Integer) (bFromSweep :type Boolean) (SweepResult :type Hit%20Result%20Structure%20%28by%20ref%29))
  ;[1 1 1] Pickup Ammo
  (bind _asfirst_person_character (Utilities|Casting|CastToFirstPersonCharacter OtherActor))
  (Variables|Default|SetFPS%20Character _asfirst_person_character)
  (Utilities|FlowControl|DoOnce false
    (:Completed
      (Audio|PlaySound2D "/Game/Audio/Item_Pickup.Item_Pickup" 1.0 1.0 0.0 0 0)
      (bind _outactors (Actor|GetAllActorsOfClass "/Game/Blueprints/BP_Glock.BP_Glock_C"))
      (Utilities|IsValid (Utilities|Array|Get(acopy) _outactors)
        (:Is%20Valid
          (Math|Integer|IncrementInt (Variables|/Game/Blueprints/BP_Glock.BP_Glock_C|GetClips (Utilities|Array|Get(acopy) _outactors))
            (:%20%20
              (Actor|DestroyActor))))
        (:Is%20Not%20Valid
          (Actor|DestroyActor))))))

(event EventTick
  (params (DeltaSeconds :type Float%20%28single-precision%29))
  ;[1 1 1] Rotate Mesh
  (Transformation|AddRelativeRotation (Variables|Default|GetStaticMesh) (Math|Rotator|MakeRotator 0.0 0.0 (* DeltaSeconds (Variables|Default|GetSpeed))) false false))

(fn ConstructionScript)