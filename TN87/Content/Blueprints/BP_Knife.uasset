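; BP_Knife is a knife weapon for the first-person character that plays its attack through the arms animation.
; BeginPlay caches the player character and its ABP_Arms animation instance.
; Fire, when neither firing nor hidden, raises the animation Blueprint's Fire flag for FireRate seconds, then clears it.
; The graph contains no hit or damage logic, and it only ever sets IsFiring to false.
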(event Custom|Fire
  ;[1 1 1] Use Weapon
  (if (and (not (Variables|Default|GetIsFiring)) (not (Variables|Rendering|GetbHidden)))
    (Variables|Default|SetIsFiring false)
    (Variables|/Game/Mesh/Arms/ABP_Arms.ABP_Arms_C|SetFire (Variables|Ref|GetArms%20Anim%20Bp) true)
    (Utilities|FlowControl|Delay (Variables|Default|GetFireRate))
    (Variables|/Game/Mesh/Arms/ABP_Arms.ABP_Arms_C|SetFire (Variables|Ref|GetArms%20Anim%20Bp) false)))

(event EventBeginPlay
  ;[1 1 1] Begin Play
  (bind _asfirst_person_character (Utilities|Casting|CastToFirstPersonCharacter (Game|GetPlayerCharacter 0)))
  (Variables|Ref|SetFPS%20Character _asfirst_person_character)
  (bind _asabp_arms (Utilities|Casting|CastToABP_Arms (Components|SkeletalMesh|GetAnimInstance (Variables|/Game/FirstPersonBP/FirstPersonCharacter.FirstPersonCharacter_C|GetPlayer_Arms _asfirst_person_character))))
  (Variables|Ref|SetArms%20Anim%20Bp _asabp_arms))

(fn ConstructionScript)