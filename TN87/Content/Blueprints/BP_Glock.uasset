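; BP_Glock is a first-person pistol with a toggleable flashlight, limited ammo and clips, and automatic reload on empty.
; On BeginPlay it caches the player character and arms anim Blueprint and enables input.
; Fire is gated by state and ammo, then drives the arms animation, a camera line trace, muzzle sound and particles, and character recoil.
; Trace hits only print the actor name; reload and flashlight sounds are print placeholders.
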(event Custom|Fire
  ;[1 1 1] Fire Weapon
  (if (Math|Boolean|ANDBoolean (not (Variables|Fire|GetIsFiring)) (Variables|Fire|GetCanFire) (> (Variables|Fire|GetAmmo) 0) (not (Variables|Rendering|GetbHidden)))
    (Utilities|FlowControl|Sequence
      (:then_0
        (Variables|Fire|SetIsFiring true)
        (Variables|/Game/Mesh/Arms/ABP_Arms.ABP_Arms_C|SetFire (Variables|Ref|GetArms_AnimBP) true)
        (Utilities|FlowControl|Delay (Variables|Fire|GetFireRate))
        (Variables|/Game/Mesh/Arms/ABP_Arms.ABP_Arms_C|SetFire (Variables|Ref|GetArms_AnimBP) false)
        (Utilities|FlowControl|Delay (Variables|Fire|GetFireRate))
        (Variables|Fire|SetIsFiring false))
      (:then_1
        ;;[1 1 1] Auto Reload
        (bind _result (Math|Integer|DecrementInt (Variables|Fire|GetAmmo))
          (:%20%20
            (if (<= _result 0)
              (CallFunction|Reload)))))
      (:then_2
        (CallFunction|Raycast)
        (CallFunction|FX)
        (Default|Recoil (Variables|Ref|GetFPS%20Character))))))

(event Custom|Raycast
  (bind _fps_character (Variables|Ref|GetFPS%20Character))
  (bind _firstpersoncamera (Variables|/Game/FirstPersonBP/FirstPersonCharacter.FirstPersonCharacter_C|GetFirstPersonCamera _fps_character))
  (bind _returnvalue (Transformation|GetWorldLocation _firstpersoncamera))
  ;[1 1 1] Raycast
  (bind (_outhit _returnvalue_2) (Collision|LineTraceByChannel _returnvalue (+ _returnvalue (* (Math|Vector|GetForwardVector (Transformation|GetWorldRotation _firstpersoncamera)) (Variables|Fire|GetRange))) "TraceTypeQuery1" false 0 "ForDuration"))
  (if _returnvalue_2
    (Development|PrintString (Utilities|GetObjectName (.HitActor (Collision|BreakHitResult _outhit))))))

(event Custom|FX
  ;[1 1 1] Spawn FX
  (Audio|PlaySoundatLocation "/Game/Audio/FirstPersonTemplateWeaponFire02.FirstPersonTemplateWeaponFire02" (Transformation|GetWorldLocation (Variables|Default|GetMuzzlePoint)) "0, 0, 0" 1.0 1.0 0.0 0 0 0)
  (bind _returnvalue (Effects|SpawnEmitterAttached "/Game/ParticleFX/Muzzle_Particle.Muzzle_Particle" (Variables|Default|GetMuzzlePoint) "None" "0, 0, 0" "0, 0, 0" "1.000000,1.000000,1.000000" "SnapToTarget"))
  (Utilities|FlowControl|Delay (Variables|Fire|GetFireRate))
  (Components|DestroyComponent _returnvalue))

(event Custom|Reload
  ;[1 1 1] Reload Weapon
  (if (not (Variables|Rendering|GetbHidden))
    (if (> (Variables|Fire|GetClips) 0)
      (Variables|Fire|SetAmmo 7)
      (Math|Integer|DecrementInt (Variables|Fire|GetClips)
        (:%20%20
          (Development|PrintString "Reload Sound")
          (Variables|Fire|SetCanFire false)
          (Utilities|FlowControl|Delay 2.0)
          (Variables|Fire|SetCanFire true))))))

(event EventBeginPlay
  ;[1 1 1] Begin Play
  (bind _asfirst_person_character (Utilities|Casting|CastToFirstPersonCharacter (Game|GetPlayerCharacter 0)))
  (Variables|Ref|SetFPS%20Character _asfirst_person_character)
  (bind _asabp_arms (Utilities|Casting|CastToABP_Arms (Components|SkeletalMesh|GetAnimInstance (Variables|/Game/FirstPersonBP/FirstPersonCharacter.FirstPersonCharacter_C|GetPlayer_Arms _asfirst_person_character))))
  (Variables|Ref|SetArms_AnimBP _asabp_arms)
  (Input|EnableInput (Game|GetPlayerController 0)))

(event Input|ActionEvents|InputActionFlashlight
  (params (Key :type Key%20Structure :default "None"))
  ;[1 1 1] Flashlight
  (:Pressed
    (Rendering|ToggleVisibility (Variables|Default|GetFlaslight) false)
    (Development|PrintString "Flashlight Sound")))

(fn ConstructionScript)