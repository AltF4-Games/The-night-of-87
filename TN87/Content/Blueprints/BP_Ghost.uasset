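; Ghost character that leaves a blood trail as it walks to a fixed spot and dies, then can be picked up for burial.
; While CanWalk is set, Tick issues AIMoveTo and a looping delayed event drops randomly rotated floor decals.
; Player overlap with its Box calls HoldBody, sets a jump-in objective, switches the first TriggerVolume to overlap pawns and destroys the ghost.
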(event OnComponentBeginOverlap(Box)
  (params (OverlappedComponent :type Primitive%20Component%20Object%20Reference) (OtherActor :type Actor%20Object%20Reference) (OtherComp :type Primitive%20Component%20Object%20Reference) (OtherBodyIndex :type Integer) (bFromSweep :type Boolean) (SweepResult :type Hit%20Result%20Structure%20%28by%20ref%29))
  ;[1 1 1] Bury The Body
  (bind _asfirst_person_character (Utilities|Casting|CastToFirstPersonCharacter OtherActor))
  (Default|HoldBody _asfirst_person_character)
  (Default|SetObjective _asfirst_person_character "Jump in loser!" 3.0)
  (bind _outactors (Actor|GetAllActorsOfClass "/Script/Engine.TriggerVolume"))
  (Utilities|IsValid (Utilities|Array|Get(acopy) _outactors)
    (:Is%20Valid
      (Collision|SetCollisionResponsetoChannel (Variables|/Script/Engine.Brush|GetBrushComponent (Utilities|Array|Get(acopy) _outactors)) "ECC_Pawn" "ECR_Overlap")
      (Actor|DestroyActor))))

(event Custom|SpawnDecals
  (bind _returnvalue (Transformation|GetActorLocation))
  (bind _returnvalue_2 (- _returnvalue "0,0.000000,90.000000"))
  ;[1 1 1] Spawn Decals
  (if (Variables|Default|GetCanWalk)
    (Rendering|Decal|SpawnDecalatLocation "/Game/RetroShadersV4/DemoContent/Environment/ColdharbourSeaside/Decals/Materials/Blood_Trail.Blood_Trail" "25.000000,100.000000,100.000000" (Math|Vector|MakeVector (.x _returnvalue_2) (.y _returnvalue_2) (.z _returnvalue_2)) (Math|Rotator|MakeRotator (Math|Random|RandomFloatinRange 0.0 3.6e+02) -9e+01 0.0) 1.8e+02))
  (Utilities|FlowControl|Delay 1.0)
  (CallFunction|SpawnDecals))

(event EventBeginPlay
  ;[1 1 1] Spawn Decals
  (CallFunction|SpawnDecals))

(event EventTick
  (params (DeltaSeconds :type Float%20%28single-precision%29))
  ;[1 1 1] Walk To Location
  (if (Variables|Default|GetCanWalk)
    (AI|AIMoveTo self "25070.000000,6800.000000, 0" 0 5.0 true
      (:OnSuccess
        (Variables|Default|SetCanWalk false)
        (Components|Movement|StopMovementImmediately (Variables|Character|GetCharacterMovement))
        (Components|Animation|PlayAnimation (Variables|Character|GetMesh) "/Game/Mesh/Ghost/Ghost_Death.Ghost_Death" false)))))

(fn ConstructionScript)