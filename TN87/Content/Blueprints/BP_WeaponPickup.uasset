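; Weapon pickup actor that shows a spinning mesh of either a Glock or a knife, chosen by the WeaponState boolean.
; On Tick the mesh rotates by Speed, and BeginPlay sets the mesh from the boolean.
; A box overlap by FirstPersonCharacter fires once, prints a placeholder sound message and flags that weapon in the character's inventory.
; It then calls the character's matching TestGlock or TestKnife function and destroys itself.
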(event OnComponentBeginOverlap(Box)
  (params (OverlappedComponent :type Primitive%20Component%20Object%20Reference) (OtherActor :type Actor%20Object%20Reference) (OtherComp :type Primitive%20Component%20Object%20Reference) (OtherBodyIndex :type Integer) (bFromSweep :type Boolean) (SweepResult :type Hit%20Result%20Structure%20%28by%20ref%29))
  ;[1 1 1] Pickup Weapon
  (bind _asfirst_person_character (Utilities|Casting|CastToFirstPersonCharacter OtherActor))
  (Variables|Default|SetFPS%20Character _asfirst_person_character)
  (Utilities|FlowControl|DoOnce false
    (:Completed
      (Development|PrintString "Pickup Sound")
      (if (Variables|Default|GetWeaponState)
        (Variables|/Game/FirstPersonBP/FirstPersonCharacter.FirstPersonCharacter_C|SetGlock_Inv (Variables|Default|GetFPS%20Character) true)
        (CallFunction|Pickup)
        (else
          (Variables|/Game/FirstPersonBP/FirstPersonCharacter.FirstPersonCharacter_C|SetKnife_Inv (Variables|Default|GetFPS%20Character) true)
          (CallFunction|Pickup))))))

(event Custom|Pickup
  (bind _fps_character (Variables|Default|GetFPS%20Character))
  ;[1 1 1] Switch to Weapon
  (if (Variables|Default|GetWeaponState)
    (Default|TestGlock _fps_character)
    (Actor|DestroyActor)
    (else
      (Default|TestKnife _fps_character)
      (Actor|DestroyActor))))

(event EventBeginPlay
  (bind _staticmesh (Variables|Default|GetStaticMesh))
  ;[1 1 1] Set Mesh
  (if (Variables|Default|GetWeaponState)
    (Components|StaticMesh|SetStaticMesh _staticmesh "/Game/Mesh/Glock/Glock.Glock")
    (else
      (Components|StaticMesh|SetStaticMesh _staticmesh "/Game/Mesh/Knife/Knife.Knife"))))

(event EventTick
  (params (DeltaSeconds :type Float%20%28single-precision%29))
  ;[1 1 1] Rotate Mesh
  (Transformation|AddLocalRotation (Variables|Default|GetStaticMesh) (Math|Rotator|MakeRotator 0.0 0.0 (* DeltaSeconds (Variables|Default|GetSpeed))) false false))

(fn ConstructionScript)